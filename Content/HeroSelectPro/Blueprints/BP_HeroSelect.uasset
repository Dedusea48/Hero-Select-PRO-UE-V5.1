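; Hero selection preview actor that loads the saved character onto its mesh at BeginPlay and stores the default rotation.
; Choosing another character reloads the mesh data, restores that rotation and plays a montage, except on a return.
; Starting selection switches to the hero camera and enables touch forwarding to the referenced widget, while returning hands control to the supplied camera.
; RotateX events spin the mesh for inspection.
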(event `self.ReceiveBeginPlay`
  ;[0 0 0] Begin Play
  (bind _codcurrentcharacter_s (`/Game/HeroSelectPro/Blueprints/BP_LibraryHeroSelect.Load Current Character`))
  (bind _selectcharacter (`/Game/HeroSelectPro/Blueprints/BP_LibraryHeroSelect.Get Data Character` _codcurrentcharacter_s))
  (`self.ChangeCharacter` _selectcharacter true)
  (bind `_rotación_relativa` (`/Game/HeroSelectPro/Blueprints/BP_LibraryRotatorCharacter.Setting Rotation` false (`self.Mesh`)))
  (set `self.RotaciónDefaultCharacter` `_rotación_relativa`))

(event `/Game/HeroSelectPro/Blueprints/BPI_Conecction.ButtonDATAUpdate`
  (params (DataCharacter :type "/Game/HeroSelectPro/Blueprints/ST_ListCharacters Structure") (codCharacter :type Integer) (`IsBlocked?` :type Boolean) (`IsReturn?` :type Boolean))
  ;[0 0 0] UpdateDataCharacter
  (`self.ChangeCharacter` DataCharacter false `IsReturn?`)
  (`/Game/HeroSelectPro/Blueprints/BP_LibraryRotatorCharacter.Setting Rotation` true (`self.Mesh`) (`self.RotaciónDefaultCharacter`)))

(event `ChangeCharacter`
  (params (ST_ListCharacters :type "/Game/HeroSelectPro/Blueprints/ST_ListCharacters Structure (by ref)") (`first time?` :type Boolean) (`isReturn?` :type Boolean))
  ;[0 0 0] UpdateDataCharacter
  (`/Game/HeroSelectPro/Blueprints/BP_LibraryHeroSelect.LoadDataCharacter` ST_ListCharacters (`self.Mesh`))
  (if (not (or `first time?` `isReturn?`))
    (`|PlayMontage` (`self.Mesh`))))

(event `/Game/HeroSelectPro/Blueprints/BPI_Conecction.StarSelectCharacter`
  (params (widgetRef :type "Widget Object Reference") (`UsedToReturn?` :type Boolean))
  ;[0 0 0] Star Selected Character
  (set `self.SystemActivated?` true)
  (`/Game/HeroSelectPro/Blueprints/BP_LibraryHeroSelect.ChangeCameraControl` (`self.HeroCamera`)))

(event `/Game/HeroSelectPro/Blueprints/BPI_Conecction.ReturnUpdateCharacter`
  (params (cameraRef :type "CameraActor Object Reference"))
  ;[0 0 0] change camera control
  (set `self.SystemActivated?` false)
  (`/Game/HeroSelectPro/Blueprints/BP_LibraryHeroSelect.ChangeCameraControl` (`CameraActor.CameraComponent` cameraRef)))

(event `/Game/HeroSelectPro/Blueprints/BPI_Rotate.RotateX`
  (params (Axis :type "Float (double-precision)"))
  ;[0 0 0] Event that adds rotation to the 3D mesh
  (`/Game/HeroSelectPro/Blueprints/BP_LibraryRotatorCharacter.MeshRotation` (`self.Mesh`) Axis 8.0))

(event `/Game/HeroSelectPro/Blueprints/BPI_Rotate.WidgetUseReference`
  (params (widgetRef :type "Widget Object Reference"))
  ;[0 0 0] Initialize the rotation system by getting the reference of the widget where it was created
  (`/Engine/EditorBlueprintResources/StandardMacros.IsValid` widgetRef
    (:`Is Valid`
      (set `self.widgetRef` widgetRef))))

(event `InputTouch`
  (params (Location :type "Vector Structure") (FingerIndex :type "ETouchIndex Enum"))
  ;[0 0 0] Get the input touch detection and notify the widget
  (:`Pressed`
    (if (`self.SystemActivated?`)
      (bind _widgetref (`self.widgetRef`)
        (:`then`
          (message `/Game/HeroSelectPro/Blueprints/BPI_Rotate.OnPressedTouch` _widgetref Location FingerIndex))
        (:`else`))))
  (:`Released`
    (if (`self.SystemActivated?`)
      (bind _widgetref_2 (`self.widgetRef`)
        (:`then`
          (message `/Game/HeroSelectPro/Blueprints/BPI_Rotate.OnReleased_Touch` _widgetref_2 Location FingerIndex))
        (:`else`))))
  (:`Moved`
    (if (`self.SystemActivated?`)
      (bind _widgetref_3 (`self.widgetRef`)
        (:`then`
          (message `/Game/HeroSelectPro/Blueprints/BPI_Rotate.OnMovedTouch` _widgetref_3 Location FingerIndex))
        (:`else`)))))

(fn `UserConstructionScript`)